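; BP_TESt is a test actor that moves ballistically under a hand-coded gravity acceleration.
; Each Tick, it draws a persistent Visibility line trace along the next step, teleport-free and unswept, then sets its location by Velocity times delta time.
; It then adds downward gravity to Velocity, an Euler integration whose debug lines leave the trajectory visible.
; The trace result is unused, so hits do not affect movement.
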(event EventBeginPlay)

(event Collision|EventActorBeginOverlap
  (params (OtherActor :type Actor%20Object%20Reference)))

(event EventTick
  (params (DeltaSeconds :type Float%20%28single-precision%29))
  (bind _returnvalue (Transformation|GetActorLocation))
  (Collision|LineTraceByChannel _returnvalue (+ _returnvalue (* (Variables|Default|GetVelocity) DeltaSeconds)) "TraceTypeQuery1" false 0 "Persistent")
  (Transformation|SetActorLocation (+ _returnvalue (* (Variables|Default|GetVelocity) DeltaSeconds)) false false)
  (Variables|Default|SetVelocity (+ (Variables|Default|GetVelocity) (* (Math|Vector|MakeVector 0.0 0.0 -9.8e+02) DeltaSeconds))))

(fn ConstructionScript)