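; BP_Jet is a jet with a CharacterMovement component and an unfinished or disconnected bombing run; all of its events are empty.
; Unwired node chains would move it forward, open a timed bombing window after a delay, and repeat a multi-bomb event while the window's flag is set.
; Another unwired node spawns BP_Bomb at a world location, so none of this logic executes.
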(event Custom|Bombing)

(event Custom|bomb%20Multi)

(event Collision|EventActorBeginOverlap
  (params (OtherActor :type Actor%20Object%20Reference)))

(event EventTick
  (params (DeltaSeconds :type Float%20%28single-precision%29)))

(event EventBeginPlay)

(fn ConstructionScript)