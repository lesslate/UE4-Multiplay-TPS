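; BP_MPPlayer is a player character Blueprint that toggles an IsAiming flag with a FlipFlop on right mouse press.
; It also holds crouch and prone stance logic, blocked while sprinting, but no event triggers either chain, so neither runs.
; Those chains zero crouched walk speed during a timed transition, then set stance-specific speed and rotation rate.
; BeginPlay, overlap, Tick and the construction script are empty.
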(event EventBeginPlay)

(event Collision|EventActorBeginOverlap
  (params (OtherActor :type Actor%20Object%20Reference)))

(event EventTick
  (params (DeltaSeconds :type Float%20%28single-precision%29)))

(event Input|ActionEvents|InputActionCrouch
  (params (Key :type Key%20Structure)))

(event Input|ActionEvents|InputActionProne
  (params (Key :type Key%20Structure)))

(event Input|MouseEvents|RightMouseButton
  (params (Key :type Key%20Structure))
  (:Pressed
    (Utilities|FlowControl|FlipFlop
      (:A
        (Variables|Default|SetIsAiming true))
      (:B
        (Variables|Default|SetIsAiming false)))))

(fn ConstructionScript)